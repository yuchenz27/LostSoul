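; Weapon Blueprint that deals melee damage to AI characters it touches.
; On actor overlap it ignores its owner and requires the owner to be attacking.
; It then casts the hit actor to AICharacter_BP, calls GetHit with WeaponDamage and prints a debug "Hit" message.
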(event `self.ReceiveActorBeginOverlap`
  (params (OtherActor :type "Actor Object Reference"))
  (bind _weaponowner (`self.WeaponOwner`))
  (`/Engine/EditorBlueprintResources/StandardMacros.IsValid` OtherActor
    (:`Is Valid`
      (`/Engine/EditorBlueprintResources/StandardMacros.IsValid` _weaponowner
        (:`Is Valid`
          (if (!= OtherActor _weaponowner)
            (if (`MainCharacter.bIsAttacking` _weaponowner)
              (bind _asaicharacter_bp (cast `/Game/Blueprints/AICharacter_BP` OtherActor))
              (`AICharacter.GetHit` _asaicharacter_bp (`self.WeaponDamage`))
              (`KismetSystemLibrary.PrintString` "Hit" true false))))))))

(fn `UserConstructionScript`)