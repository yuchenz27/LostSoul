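; Behavior Tree service that records how far the AI-controlled pawn is from its combat target.
; On activation only, with no tick update, it reads CombatTarget from the Blackboard and stops unless that is a MainCharacter_BP.
; It writes the distance to CombatTargetDistance, then compares it against ObservingRange and MeleeRange to set the IsInObservingRange and IsInMeleeRange flags.
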(event `self.ReceiveActivationAI`
  (params (OwnerController :type "AIController Object Reference") (ControlledPawn :type "Pawn Object Reference"))
  (bind _asmain_character_bp (cast `/Game/Blueprints/MainCharacter_BP` (`BTFunctionLibrary.GetBlackboardValueAsObject` (`self.CombatTarget`))))
  (bind _returnvalue (`KismetMathLibrary.Vector_Distance` (`Actor.K2_GetActorLocation` _asmain_character_bp) (`Actor.K2_GetActorLocation` ControlledPawn)))
  (`BTFunctionLibrary.SetBlackboardValueAsFloat` (`self.CombatTargetDistance`) _returnvalue)
  (`BTFunctionLibrary.SetBlackboardValueAsBool` (`self.IsInObservingRange`) (< _returnvalue (`self.ObservingRange`)))
  (`BTFunctionLibrary.SetBlackboardValueAsBool` (`self.IsInMeleeRange`) (< _returnvalue (`self.MeleeRange`))))