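; ObservingMove is a Behavior Tree task that makes an AICharacter_BP strafe briefly left or right, judging by the movement states it sets.
; It picks MovingLeft or MovingRight from the LeftOrRight blackboard bool, holds it for a fixed delay, then sets NotMoving.
; It then randomizes that bool for the next run and finishes successfully; a failed pawn cast never calls FinishExecute.
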(event `self.ReceiveExecuteAI`
  (params (OwnerController :type "AIController Object Reference") (ControlledPawn :type "Pawn Object Reference"))
  (bind _asaicharacter_bp (cast `/Game/Blueprints/AICharacter_BP` ControlledPawn))
  (if (`BTFunctionLibrary.GetBlackboardValueAsBool` (`self.LeftOrRight`))
    (set `AICharacter.AIMovementStatus` "AMS_MovingLeft" _asaicharacter_bp)
    (else
      (set `AICharacter.AIMovementStatus` "AMS_MovingRight" _asaicharacter_bp)))
  (`KismetSystemLibrary.Delay` 1.5)
  (set `AICharacter.AIMovementStatus` "AMS_NotMoving" _asaicharacter_bp)
  (`BTFunctionLibrary.SetBlackboardValueAsBool` (`self.LeftOrRight`) (`KismetMathLibrary.RandomBool`))
  (`self.FinishExecute` true))