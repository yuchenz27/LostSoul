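; Player character with a three-hit sword combo, walk/run/sprint switching, target lock-on and HUD creation.
; Clicks during attacks are buffered until ComboAttackSave plays the next montage section; ResetCombo clears the chain, and sword overlaps damage AICharacter_BP.
; Lock-on picks the closest line-of-sight AI within range and toggles a gate for yaw-only camera tracking.
; That gate is entered only from a Timeline update marked as never run.
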(event `self.ReceiveBeginPlay`
  ;[1 1 1] HUD initialization
  (bind _returnvalue (`|CreateWidget` "/Game/HUD/HUDOverlay.HUDOverlay_C" (`GameplayStatics.GetPlayerController` 0)))
  (`UserWidget.AddToViewport` _returnvalue 0)
  ;[1 1 1] Set sword default collision
  (`PrimitiveComponent.SetCollisionEnabled` (`self.Sword`) "NoCollision"))

(event `Key|LeftMouseButton`
  (params (Key :type "Key Structure"))
  (bind _returnvalue (`SkeletalMeshComponent.GetAnimInstance` (`self.Mesh`)))
  ;[1 1 1] Attack Combo
  (:`Pressed`
    (if (`self.IsAttacking`)
      (set `self.SaveAttack` true)
      (else
        (set `self.IsAttacking` true)
        (switch `int` (`self.AttackCount`) :!label _label
          (:`0`
            (set `self.AttackCount` 1)
            (`AnimInstance.Montage_Play` _returnvalue "/Game/Rapier_AnimSet/Animation/Montages/Combo_Montage.Combo_Montage" 0.8 "MontageLength" 0.0 true)
            (`AnimInstance.Montage_JumpToSection` _returnvalue "Attack0" "/Game/Rapier_AnimSet/Animation/Montages/Combo_Montage.Combo_Montage"))
          (:`1`
            (set `self.AttackCount` 2)
            (`AnimInstance.Montage_Play` _returnvalue "/Game/Rapier_AnimSet/Animation/Montages/Combo_Montage.Combo_Montage" 0.8 "MontageLength" 0.0 true)
            (`AnimInstance.Montage_JumpToSection` _returnvalue "Attack1" "/Game/Rapier_AnimSet/Animation/Montages/Combo_Montage.Combo_Montage"))
          (:`2`
            (set `self.AttackCount` 0)
            (`AnimInstance.Montage_Play` _returnvalue "/Game/Rapier_AnimSet/Animation/Montages/Combo_Montage.Combo_Montage" 0.8 "MontageLength" 0.0 true)
            (`AnimInstance.Montage_JumpToSection` _returnvalue "Attack2" "/Game/Rapier_AnimSet/Animation/Montages/Combo_Montage.Combo_Montage")))))))

(event `ComboAttackSave`
  ;[1 1 1] Attack Combo
  (if (`self.SaveAttack`)
    (set `self.SaveAttack` false)
    (goto _label)))

(event `ResetCombo`
  ;[1 1 1] Attack Combo
  (set `self.AttackCount` 0)
  (set `self.SaveAttack` false)
  (set `self.IsAttacking` false))

(event `Key|LeftControl`
  (params (Key :type "Key Structure"))
  (bind _movementstatus (`self.MovementStatus`))
  (bind _charactermovement (`self.CharacterMovement`))
  ;[1 1 1] Walk/Run/Sprint
  (:`Pressed`
    (if (`|EnumInequality` _movementstatus "MS_Sprint")
      (if (`|EnumEquality` _movementstatus "MS_Walk")
        (set `self.MovementStatus` "MS_Run")
        (set `CharacterMovementComponent.MaxWalkSpeed` 600.0 _charactermovement)
        (else
          (set `self.MovementStatus` "MS_Walk")
          (set `CharacterMovementComponent.MaxWalkSpeed` 300.0 _charactermovement))))))

(event `Key|LeftShift`
  (params (Key :type "Key Structure"))
  (bind _movementstatus (`self.MovementStatus`))
  (bind _charactermovement (`self.CharacterMovement`))
  ;[1 1 1] Walk/Run/Sprint
  (:`Pressed`
    (if (`|EnumEquality` _movementstatus "MS_Run")
      (set `self.MovementStatus` "MS_Sprint")
      (set `CharacterMovementComponent.MaxWalkSpeed` 900.0 _charactermovement)))
  (:`Released`
    (if (`|EnumEquality` _movementstatus "MS_Sprint")
      (set `self.MovementStatus` "MS_Run")
      (set `CharacterMovementComponent.MaxWalkSpeed` 600.0 _charactermovement))))

(event `self.Sword.OnComponentBeginOverlap`
  (params (OverlappedComponent :type "PrimitiveComponent Object Reference") (OtherActor :type "Actor Object Reference") (OtherComp :type "PrimitiveComponent Object Reference") (OtherBodyIndex :type Integer) (bFromSweep :type Boolean) (SweepResult :type "HitResult Structure (by ref)"))
  ;[1 1 1] Hit the enemy
  (bind _asaicharacter_bp (cast `/Game/Blueprints/AICharacter_BP` OtherActor))
  (`/Game/Blueprints/AICharacter_BP.OnHit` _asaicharacter_bp (`self.K2_GetActorLocation`) 13.0)
  (`KismetSystemLibrary.PrintString` "Player hit AI"))

(event `InputAction|Target`
  (params (Key :type "Key Structure"))
  ;[1 1 1] Lock on/off the target
  (:`Pressed`
    (set `self.ClosestTargetDistance` (`self.MinimumDistanceToEnable`))
    (if (`self.TargetLocked`)
      (set `self.TargetLocked` false)
      (message `/Game/Blueprints/TargetingSystem_BPI.TargetLockOn` (`self.NearestTarget`) :!label _label_2)
      (`/Engine/EditorBlueprintResources/StandardMacros.Gate` true :!via `Toggle`
        (:`Exit`
          ;[1 1 1] Camera following locked target
          (`Controller.SetControlRotation` (`self.GetController`) (`KismetMathLibrary.MakeRotator` (.roll (`self.GetControlRotation`)) (.pitch (`self.GetControlRotation`)) (.yaw (`KismetMathLibrary.RInterpTo` (struct) (`KismetMathLibrary.FindLookAtRotation` (`SceneComponent.K2_GetComponentLocation` (`self.FollowCamera`)) (`self.K2_GetActorLocation` (`self.NearestTarget`))) (`GameplayStatics.GetWorldDeltaSeconds`)))))))
      (else
        (bind _outactors (`GameplayStatics.GetAllActorsOfClass` "/Game/Blueprints/AICharacter_BP.AICharacter_BP_C"))
        (for _array_element _outactors
          (bind _outhit (`KismetSystemLibrary.LineTraceSingleForObjects` (`self.K2_GetActorLocation`) (`self.K2_GetActorLocation` _array_element) (`|MakeArray` "ObjectTypeQuery1" "ObjectTypeQuery2" "ObjectTypeQuery3" :!type "EObjectTypeQuery Enum")))
          (if (== _array_element (`.HitActor` (`GameplayStatics.BreakHitResult` _outhit)))
            (bind _distancefromplayer (`/Game/Blueprints/AICharacter_BP.ComputeDistanceFromPlayer` _array_element))
            (`/Engine/EditorBlueprintResources/StandardMacros.CompareFloat` _distancefromplayer (`self.ClosestTargetDistance`)
              (:`<`
                (set `self.ClosestTargetDistance` _distancefromplayer)
                (set `self.NearestTarget` _array_element)))))
        (if (< (`self.ClosestTargetDistance`) (`self.MinimumDistanceToEnable`))
          (set `self.TargetLocked` true)
          (goto _label_2))))))

(fn `UserConstructionScript`)